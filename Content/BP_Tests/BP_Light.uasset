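; BP_Light is an interactable spotlight actor that the player can switch on and off with the F key while standing inside its trigger box.
; Entering or leaving the box enables or disables input for player 0 and toggles the visibility of a help text.
; The construction script applies the configurable light color and initial visibility to the spotlight.
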(event `self.TiggerBox.OnComponentBeginOverlap`
  (params (OverlappedComponent :type "PrimitiveComponent Object Reference") (OtherActor :type "Actor Object Reference") (OtherComp :type "PrimitiveComponent Object Reference") (OtherBodyIndex :type Integer) (bFromSweep :type Boolean) (SweepResult :type "HitResult Structure (by ref)"))
  ;[0.5431 0.6714 1] Entering the TriggerBox, enables input and turns on visibility of HelpfulText. Whereas leaving the TriggerBox, disables input and turns off the HelpfulText.
  (`self.EnableInput` (`GameplayStatics.GetPlayerController` 0))
  (`SceneComponent.ToggleVisibility` (`self.HelpfulText`) false :!label _label))

(event `self.TiggerBox.OnComponentEndOverlap`
  (params (OverlappedComponent :type "PrimitiveComponent Object Reference") (OtherActor :type "Actor Object Reference") (OtherComp :type "PrimitiveComponent Object Reference") (OtherBodyIndex :type Integer))
  ;[0.5431 0.6714 1] Entering the TriggerBox, enables input and turns on visibility of HelpfulText. Whereas leaving the TriggerBox, disables input and turns off the HelpfulText.
  (`self.DisableInput` (`GameplayStatics.GetPlayerController` 0))
  (goto _label))

(event `Key|F`
  (params (Key :type "Key Structure"))
  ;[1 0.9023 0.6979] Press F to toggle SpotLight
  (:`Pressed`
    (`SceneComponent.ToggleVisibility` (`self.SpotLight`) false)))

(fn `UserConstructionScript`
  (bind _spotlight (`self.SpotLight`))
  (`LightComponent.SetLightColor` _spotlight (`self.Light Color`) true)
  (`SceneComponent.SetVisibility` _spotlight (`self.Visibility Setting`) false))