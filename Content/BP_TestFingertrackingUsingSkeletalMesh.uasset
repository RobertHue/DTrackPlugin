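; Test actor for driving a skeletal mesh from hand and finger tracking, currently only visualizing the tracked hand pose.
; Each hand tracking event spawns a small crosshair at the translation offset by the mesh's world location, marking the intended IK end effector target.
; Each marker's lifespan is the Tick delta time, so it lasts about one frame.
; Index finger bone rotation from tracking data is present but unconnected.
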(event `self.ReceiveTick`
  (params (DeltaSeconds :type "Float (single-precision)")))

(event `DTrackInterface.OnHandTracking`
  (params (HandID :type Integer) (Right :type Boolean) (Translation :type "Vector Structure (by ref)") (Rotation :type "Rotator Structure (by ref)") (Fingers :type "Array of DTrackFinger Structure (by ref)"))
  ;[1 1 1] INDEX: Indicator showing the end effector target positons for the IK of the Hand
  (bind _returnvalue (`|SpawnActorFromClass` "/DTrackPlugin/BP_Helpers/BP_Crosshair_SpawnAtLocation.BP_Crosshair_SpawnAtLocation_C" (`KismetMathLibrary.MakeTransform` (+ Translation (`SceneComponent.K2_GetComponentLocation` (`self.SkeletalMeshComponent`))) Rotation (0.05 0.05 0.05)) "Undefined" "OverrideRootScale" null null))
  (`self.SetLifeSpan` _returnvalue (* (stale `self.ReceiveTick` DeltaSeconds) 1.0)))

(fn `UserConstructionScript`)