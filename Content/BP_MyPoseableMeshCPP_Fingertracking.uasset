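; Debug-visualization Blueprint for finger tracking, showing the right hand's IK end-effector targets.
; Each Tick spawns small crosshair actors at the five fingertip target transforms and a larger one at the hand transform.
; Each marker's lifespan equals the frame's delta time, so markers are respawned every frame rather than moved.
; Unconnected debug chains for thumb bone rotation, an axis cube and per-bone rotation markers never run.
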(event `self.ReceiveTick`
  (params (DeltaSeconds :type "Float (single-precision)"))
  (bind _returnvalue (* DeltaSeconds 1.0))
  ;[1 1 1] INDEX: Indicator showing the end effector target positons for the IK of the Hand
  (bind _returnvalue_2 (`|SpawnActorFromClass` "/DTrackPlugin/BP_Helpers/BP_Crosshair_SpawnAtLocation.BP_Crosshair_SpawnAtLocation_C" (`KismetMathLibrary.MakeTransform` (`|GetArrayItem` (`self.m_HandREndEffectorLocations`) 1) (`|GetArrayItem` (`self.m_HandREndEffectorRotators`) 1) (0.05 0.05 0.05)) "Undefined" "OverrideRootScale" null null))
  (`self.SetLifeSpan` _returnvalue_2 _returnvalue)
  ;[1 1 1] MIDDLE: Indicator showing the end effector target positons for the IK of the Hand
  (bind _returnvalue_3 (`|SpawnActorFromClass` "/DTrackPlugin/BP_Helpers/BP_Crosshair_SpawnAtLocation.BP_Crosshair_SpawnAtLocation_C" (`KismetMathLibrary.MakeTransform` (`|GetArrayItem` (`self.m_HandREndEffectorLocations`) 2) (`|GetArrayItem` (`self.m_HandREndEffectorRotators`) 2) (0.05 0.05 0.05)) "Undefined" "OverrideRootScale" null null))
  (`self.SetLifeSpan` _returnvalue_3 _returnvalue)
  ;[1 1 1] THUMB: Indicator showing the end effector target positons for the IK of the Hand
  (bind _returnvalue_4 (`|SpawnActorFromClass` "/DTrackPlugin/BP_Helpers/BP_Crosshair_SpawnAtLocation.BP_Crosshair_SpawnAtLocation_C" (`KismetMathLibrary.MakeTransform` (`|GetArrayItem` (`self.m_HandREndEffectorLocations`)) (`|GetArrayItem` (`self.m_HandREndEffectorRotators`)) (0.05 0.05 0.05)) "Undefined" "OverrideRootScale" null null))
  (`self.SetLifeSpan` _returnvalue_4 _returnvalue)
  ;[1 1 1] RING: Indicator showing the end effector target positons for the IK of the Hand
  (bind _returnvalue_5 (`|SpawnActorFromClass` "/DTrackPlugin/BP_Helpers/BP_Crosshair_SpawnAtLocation.BP_Crosshair_SpawnAtLocation_C" (`KismetMathLibrary.MakeTransform` (`|GetArrayItem` (`self.m_HandREndEffectorLocations`) 3) (`|GetArrayItem` (`self.m_HandREndEffectorRotators`) 3) (0.05 0.05 0.05)) "Undefined" "OverrideRootScale" null null))
  (`self.SetLifeSpan` _returnvalue_5 _returnvalue)
  ;[1 1 1] PINKY: Indicator showing the end effector target positons for the IK of the Hand
  (bind _returnvalue_6 (`|SpawnActorFromClass` "/DTrackPlugin/BP_Helpers/BP_Crosshair_SpawnAtLocation.BP_Crosshair_SpawnAtLocation_C" (`KismetMathLibrary.MakeTransform` (`|GetArrayItem` (`self.m_HandREndEffectorLocations`) 4) (`|GetArrayItem` (`self.m_HandREndEffectorRotators`) 4) (0.05 0.05 0.05)) "Undefined" "OverrideRootScale" null null))
  (`self.SetLifeSpan` _returnvalue_6 _returnvalue)
  ;[1 1 1] INDEX: Indicator showing the end effector target positons for the IK of the Hand
  (bind _returnvalue_7 (`|SpawnActorFromClass` "/DTrackPlugin/BP_Helpers/BP_Crosshair_SpawnAtLocation.BP_Crosshair_SpawnAtLocation_C" (`KismetMathLibrary.MakeTransform` (`self.m_HandLocation`) (`self.m_HandRotator`) (0.1 0.1 0.1)) "Undefined" "OverrideRootScale" null null))
  (`self.SetLifeSpan` _returnvalue_7 _returnvalue))

(fn `UserConstructionScript`)